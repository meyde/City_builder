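; BP_Mobile is an actor that wanders along road cells of the BP_GridManager grid, like a vehicle.
; Each tick it moves toward its destination at Speed, snapping on arrival and then choosing the next cell.
; ChoseNextCell picks a random adjacent road cell, backtracking only at dead ends, and destroys the actor if its current cell is not road.
; Destinations are shifted perpendicular to travel by Offset to keep a lane side, and the actor turns to face them.
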(event `self.ReceiveBeginPlay`
  (bind _returnvalue (`GameplayStatics.GetActorOfClass` "/Game/Game/BP/Grid/BP_GridManager.BP_GridManager_C"))
  (bind _output_get (set `self.Grid` _returnvalue))
  (bind _cell (`/Game/Game/BP/Grid/BP_GridManager.WorldToGrid` _output_get (`self.K2_GetActorLocation`)))
  (bind _output_get_2 (set `self.CurrentCell` _cell))
  (set `self.PreviousCell` _output_get_2)
  (`self.ChoseNextCell`))

(event `self.ReceiveTick`
  (params (DeltaSeconds :type "Float (single-precision)"))
  (bind _returnvalue (`self.K2_GetActorLocation`))
  (bind _destination (`self.Destination`))
  (bind _returnvalue_2 (* DeltaSeconds (`self.Speed`)))
  (if (<= (`KismetMathLibrary.Vector_Distance` _destination _returnvalue) _returnvalue_2)
    (`self.K2_SetActorLocation` (`self.Destination`))
    (set `self.PreviousCell` (`self.CurrentCell`))
    (set `self.CurrentCell` (`self.NextCell`))
    (`self.ChoseNextCell`)
    (else
      (`self.K2_AddActorWorldOffset` (* (`KismetMathLibrary.Normal` (- _destination _returnvalue)) _returnvalue_2)))))

(fn `ChoseNextCell`
  (bind _road (`/Game/Game/BP/Grid/BP_GridManager.IsRoad` (`self.Grid`) (`self.CurrentCell`)))
  (if _road
    (`KismetArrayLibrary.Array_Clear` (`self.Candidates`))
    (for _array_element (`/Game/Game/BP/Grid/BP_GridManager.Directions` (`self.Grid`))
      (bind _returnvalue (+ _array_element (`self.CurrentCell`)))
      (bind _road_2 (`/Game/Game/BP/Grid/BP_GridManager.IsRoad` (`self.Grid`) _returnvalue))
      (if (and _road_2 (not (`KismetMathLibrary.Equal_IntPointIntPoint` _returnvalue (`self.PreviousCell`))))
        (`KismetArrayLibrary.Array_Add` (`self.Candidates`) _returnvalue)))
    (`|ExecutionSequence`
      (:`then_0`
        (if (`KismetArrayLibrary.Array_IsEmpty` (`self.Candidates`))
          (`KismetArrayLibrary.Array_Add` (`self.Candidates`) (`self.PreviousCell`))))
      (:`then_1`
        (set `self.NextCell` (`KismetArrayLibrary.Array_Random` (`self.Candidates`)))
        (bind _position (`/Game/Game/BP/Grid/BP_GridManager.GridToWorld` (`self.Grid`) (`self.CurrentCell`)))
        (bind _position_2 (`/Game/Game/BP/Grid/BP_GridManager.GridToWorld` (`self.Grid`) (`self.NextCell`)))
        (bind (_returnvalue_x _returnvalue_y) (`KismetMathLibrary.BreakVector` (`KismetMathLibrary.Normal` (- _position_2 _position))))
        (set `self.Destination` (+ _position_2 (* (`KismetMathLibrary.MakeVector` (* _returnvalue_y -1.0) _returnvalue_x) (`self.Offset`))))
        (`self.K2_SetActorRotation` (`KismetMathLibrary.FindLookAtRotation` (`self.K2_GetActorLocation`) (`self.Destination`)))))
    (else
      (`self.K2_DestroyActor`))))

(fn `UserConstructionScript`)
(event `self.ReceiveBeginPlay`
  (`EnhancedInputSubsystemInterface.AddMappingContext` (subsystem `EnhancedInputLocalPlayerSubsystem`) "/Game/Game/Input/IMC_Default.IMC_Default" 0 (struct))
  (bind _returnvalue (`GameplayStatics.GetActorOfClass` "/Game/Game/BP/Grid/BP_GridManager.BP_GridManager_C"))
  (set `self.GridManager` _returnvalue)
  (bind _asbp_game_mode (cast `/Game/Game/BP/Core/BP_GameMode` (`GameplayStatics.GetGameMode`)))
  (set `self.MyGameMode` _asbp_game_mode)
  (bind _returnvalue_2 (`|CreateWidget` "/Game/Game/UI/WBP_HUD.WBP_HUD_C"))
  (`UserWidget.AddToViewport` _returnvalue_2 0))

(event `self.ReceiveTick`
  (params (DeltaSeconds :type "Float (single-precision)"))
  (bind (_hitresult _returnvalue) (`self.GetHitResultUnderCursorByChannel` "TraceTypeQuery1" false))
  (if _returnvalue
    (bind _cell (`/Game/Game/BP/Grid/BP_GridManager.WorldToGrid` (`self.GridManager`) (`.ImpactPoint` (`GameplayStatics.BreakHitResult` _hitresult))))
    (bind _output_get (set `self.HoveredCell` _cell))
    (`/Game/Game/BP/Grid/BP_GridManager.ShowCell` (`self.GridManager`) _output_get)))

(event `EnhancedInput|/Game/Game/Input/Action/IA_Build`
  (params (ActionValue :type Boolean) (ElapsedSeconds :type "Float (double-precision)") (TriggeredSeconds :type "Float (double-precision)") (InputAction :type "InputAction Object Reference" :default "/Game/Game/Input/Action/IA_Build.IA_Build"))
  (:`Started`
    (bind _ok (`/Game/Game/BP/Grid/BP_GridManager.CanBuild` (`self.GridManager`) (`self.HoveredCell`)))
    (if _ok
      (bind _returnvalue (`|GetDataTableRow` "/Game/Game/Data/DT_Buildings.DT_Buildings" (`self.SelectedBuilding`))
        (:`then`
          (bind _ok_2 (`/Game/Game/BP/Core/BP_GameMode.Pay` (`self.MyGameMode`) (`.Cost_9_0C69A27B49463710E0632C8367228CBD` (break `/Game/Game/Data/S_Building` _returnvalue))))
          (if _ok_2
            (bind _position (`/Game/Game/BP/Grid/BP_GridManager.GridToWorld` (`self.GridManager`) (`self.HoveredCell`)))
            (bind _returnvalue_2 (`|SpawnActorFromClass` (`.Class_14_5A4B7CBD466EE8B633680AB98EABDE1E` (break `/Game/Game/Data/S_Building` _returnvalue)) (`KismetMathLibrary.Conv_VectorToTransform` _position) "Undefined" "MultiplyWithRoot" null (`self.HoveredCell`) (`self.SelectedBuilding`) null))
            (`/Game/Game/BP/Grid/BP_GridManager.OccupyCell` (`self.GridManager`) (`self.HoveredCell`) _returnvalue_2)))))))

(event `EnhancedInput|/Game/Game/Input/Action/IA_Destroy`
  (params (ActionValue :type Boolean) (ElapsedSeconds :type "Float (double-precision)") (TriggeredSeconds :type "Float (double-precision)") (InputAction :type "InputAction Object Reference" :default "/Game/Game/Input/Action/IA_Destroy.IA_Destroy"))
  (:`Started`
    (`/Game/Game/BP/Grid/BP_GridManager.FreeCell` (`self.GridManager`) (`self.HoveredCell`))))

(fn `UserConstructionScript`)
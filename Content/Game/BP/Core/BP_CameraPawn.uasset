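; BP_CameraPawn is a player camera pawn that moves, rotates and zooms over the map through Enhanced Input actions.
; Move input pushes the pawn along its forward and right vectors, and rotate input yaws it at a frame-rate-independent speed.
; Zoom input sets a clamped target that Tick eases the spring arm length toward.
; Tick also clamps X and Y position to a square map limit centred on the origin.
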(event `EnhancedInput|/Game/Game/Input/Action/IA_Move`
  (params (ActionValue :type "Vector2D Structure") (ElapsedSeconds :type "Float (double-precision)") (TriggeredSeconds :type "Float (double-precision)") (InputAction :type "InputAction Object Reference" :default "/Game/Game/Input/Action/IA_Move.IA_Move"))
  (bind (_x _y) (`KismetMathLibrary.BreakVector2D` ActionValue))
  (:`Triggered`
    (`self.AddMovementInput` (`self.GetActorForwardVector`) _y)
    (`self.AddMovementInput` (`self.GetActorRightVector`) _x)))

(event `EnhancedInput|/Game/Game/Input/Action/IA_Rotate`
  (params (ActionValue :type "Float (double-precision)") (ElapsedSeconds :type "Float (double-precision)") (TriggeredSeconds :type "Float (double-precision)") (InputAction :type "InputAction Object Reference" :default "/Game/Game/Input/Action/IA_Rotate.IA_Rotate"))
  (:`Triggered`
    (`self.K2_AddActorWorldRotation` (`KismetMathLibrary.MakeRotator` 0.0 0.0 (* (* ActionValue (`self.Rotation Speed`)) (`GameplayStatics.GetWorldDeltaSeconds`))))))

(event `EnhancedInput|/Game/Game/Input/Action/IA_Zoom`
  (params (ActionValue :type "Float (double-precision)") (ElapsedSeconds :type "Float (double-precision)") (TriggeredSeconds :type "Float (double-precision)") (InputAction :type "InputAction Object Reference" :default "/Game/Game/Input/Action/IA_Zoom.IA_Zoom"))
  (:`Triggered`
    (set `self.TargetZoom` (`KismetMathLibrary.FClamp` (- (`self.TargetZoom`) (* ActionValue (`self.Zoom scale`))) (`self.Max Camera Zoom`) (`self.Min Camera Zoom`)))))

(event `self.ReceiveTick`
  (params (DeltaSeconds :type "Float (single-precision)"))
  (bind (_returnvalue_x _returnvalue_y _returnvalue_z) (`KismetMathLibrary.BreakVector` (`self.K2_GetActorLocation`)))
  (bind _returnvalue (* (`self.MapLimit`) -1.0))
  (set `SpringArmComponent.TargetArmLength` (`KismetMathLibrary.FInterpTo` (`SpringArmComponent.TargetArmLength` (`self.SpringArm`)) (`self.TargetZoom`) (`GameplayStatics.GetWorldDeltaSeconds`) 8.0) (`self.SpringArm`))
  (`self.K2_SetActorLocation` (`KismetMathLibrary.MakeVector` (`KismetMathLibrary.FClamp` _returnvalue_x _returnvalue (`self.MapLimit`)) (`KismetMathLibrary.FClamp` _returnvalue_y _returnvalue (`self.MapLimit`)) _returnvalue_z)))

(fn `UserConstructionScript`)
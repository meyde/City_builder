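; BP_GameMode runs a city-builder economy and ambient traffic on looping timers started at BeginPlay.
; A city count rebuilds income, population and happiness totals from every BP_Building, and income collection adds to Money, halved while happiness is negative.
; Traffic spawning creates a random car or pedestrian at a random BP_Road while the BP_Mobile count is below a cap.
; Pay deducts an affordable amount and reports success.
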(event `SpawnTraffic`
  (bind _outactors (`GameplayStatics.GetAllActorsOfClass` "/Game/Game/BP/Mobile/BP_Mobile.BP_Mobile_C"))
  (if (< (`KismetArrayLibrary.Array_Length` _outactors) 30)
    (bind _outactors_2 (`GameplayStatics.GetAllActorsOfClass` "/Game/Game/BP/Buildings/BP_Road.BP_Road_C"))
    (if (`KismetArrayLibrary.Array_IsNotEmpty` _outactors_2)
      (if (`KismetMathLibrary.RandomBool`)
        (bind _returnvalue (`KismetMathLibrary.Conv_VectorToTransform` (`self.K2_GetActorLocation` (`KismetArrayLibrary.Array_Random` _outactors_2))))
        (`|SpawnActorFromClass` "/Game/Game/BP/Mobile/BP_Car.BP_Car_C" _returnvalue "Undefined" "MultiplyWithRoot" null null)
        (else
          (`|SpawnActorFromClass` "/Game/Game/BP/Mobile/BP_Pedestrian.BP_Pedestrian_C" _returnvalue "Undefined" "MultiplyWithRoot" null null))))))

(event `self.ReceiveBeginPlay`
  (`KismetSystemLibrary.K2_SetTimerDelegate` (delegate `CollectIncome`) (`self.IncomeGatheringSpeed`) true)
  (`KismetSystemLibrary.K2_SetTimerDelegate` (delegate `SpawnTraffic`) (`self.MobileSpawnDelay`) true)
  (`KismetSystemLibrary.K2_SetTimerDelegate` (delegate `CountCity`) 0.5 true))

(event `CollectIncome`
  (if (>= (`self.Hapiness`) 0)
    (set `self.money` (+ (`self.money`) (`self.IncomePerCycle`)))
    (else
      (set `self.money` (+ (`self.money`) (/ (`self.IncomePerCycle`) 2))))))

(event `CountCity`
  (set `self.IncomePerCycle` 0)
  (set `self.Population` 0)
  (set `self.Hapiness` 0)
  (bind _outactors (`GameplayStatics.GetAllActorsOfClass` "/Game/Game/BP/Buildings/BP_Building.BP_Building_C"))
  (for _array_element _outactors
    (bind _income (`/Game/Game/BP/Buildings/BP_Building.GetIncome` _array_element))
    (set `self.IncomePerCycle` (+ _income (`self.IncomePerCycle`)))
    (bind _residents (`/Game/Game/BP/Buildings/BP_Building.GetResident` _array_element))
    (set `self.Population` (+ _residents (`self.Population`)))
    (bind _hapiness (`/Game/Game/BP/Buildings/BP_Building.GetHapiness` _array_element))
    (set `self.Hapiness` (+ _hapiness (`self.Hapiness`)))))

(fn `Pay`
  (params (Amount :type Integer))
  (returns (Ok :type Boolean))
  (if (<= Amount (`self.money`))
    (set `self.money` (- (`self.money`) Amount))
    (return true)
    (else
      (return false))))

(fn `UserConstructionScript`)
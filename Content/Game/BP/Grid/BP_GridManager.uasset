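; Grid manager for a building placement game that spawns an instanced mesh for every cell and converts between world positions and cell coordinates.
; An occupancy map links cells to placed buildings and roads, driving build validity, lookups and removal.
; Occupying or freeing a cell makes that cell and its neighboring roads update their shape.
; It also positions a green or red cell highlight and a rotatable mesh preview.
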(event `self.ReceiveBeginPlay`
  (for _index (range (`self.CellCountX`))
    (for _index_2 (range (`self.CellCountY`))
      (bind _position (`self.GridToWorld` (make `IntPoint` _index _index_2)))
      (`InstancedStaticMeshComponent.AddInstance` (`self.Cells`) (`KismetMathLibrary.MakeTransform` _position (struct) (0.95 0.95 1.0)) true))))

(fn `CanBuild`
  (params (Cell :type "IntPoint Structure"))
  (returns (Ok :type Boolean))
  (bind _inside (`self.IsInsideGrid` Cell))
  (return (and _inside (not (`BlueprintMapLibrary.Map_Contains` (`self.Occupancy`) Cell)))))

(fn `FreeCell`
  (params (Cell :type "IntPoint Structure"))
  (bind _value (`BlueprintMapLibrary.Map_Find` (`self.Occupancy`) Cell))
  (`/Engine/EditorBlueprintResources/StandardMacros.IsValid` _value
    (:`Is Valid`
      (`self.K2_DestroyActor` _value)
      (`BlueprintMapLibrary.Map_Remove` (`self.Occupancy`) Cell)
      (`self.RefreshNeighbors` Cell))))

(fn `GetBuildingAt`
  (params (Cell :type "IntPoint Structure"))
  (returns (Building :type "/Game/Game/BP/Buildings/BP_Building Object Reference"))
  (return (cast `/Game/Game/BP/Buildings/BP_Building` (`BlueprintMapLibrary.Map_Find` (`self.Occupancy`) Cell) :!pure true)))

(fn `GridToWorld`
  (params (Cell :type "IntPoint Structure"))
  (returns (Position :type "Vector Structure"))
  (bind (_returnvalue_x _returnvalue_y) (`KismetMathLibrary.BreakVector` (`self.K2_GetActorLocation`)))
  (bind _returnvalue (/ (`self.CellSize`) 2.0))
  (return (`KismetMathLibrary.MakeVector` (+ (* Cell_X (`self.CellSize`)) _returnvalue_x _returnvalue) (+ _returnvalue_y _returnvalue (* Cell_Y (`self.CellSize`))))))

(fn `HasRoadNeighbor`
  (params (Cell :type "IntPoint Structure"))
  (returns (Connected :type Boolean))
  (for _array_element (`self.Directions`)
    (bind _road (`self.IsRoad` (+ _array_element Cell)))
    (if _road
      (return true)))
  (return false))

(fn `IsInsideGrid`
  (params (Cell :type "IntPoint Structure"))
  (returns (Inside :type Boolean))
  (bind (_x _y) (break `IntPoint` Cell))
  (return (and (>= _x 0) (< _x (`self.CellCountX`)) (>= _y 0) (< _y (`self.CellCountY`)))))

(fn `IsRoad`
  (params (Cell :type "IntPoint Structure"))
  (returns (Road :type Boolean))
  (return (`.bSuccess` (cast `/Game/Game/BP/Buildings/BP_Road` (`BlueprintMapLibrary.Map_Find` (`self.Occupancy`) Cell) :!pure true))))

(fn `OccupyCell`
  (params (Cell :type "IntPoint Structure") (Building :type "Actor Object Reference"))
  (`BlueprintMapLibrary.Map_Add` (`self.Occupancy`) Cell Building)
  (`self.RefreshNeighbors` Cell))

(fn `Refresh Cell`
  (params (Cell :type "IntPoint Structure"))
  (bind _asbp_road (cast `/Game/Game/BP/Buildings/BP_Road` (`BlueprintMapLibrary.Map_Find` (`self.Occupancy`) Cell)))
  (`/Game/Game/BP/Buildings/BP_Road.UpdateShape` _asbp_road self))

(fn `RefreshNeighbors`
  (params (Cell :type "IntPoint Structure"))
  (`self.Refresh Cell` Cell)
  (for _array_element (`self.Directions`)
    (`self.Refresh Cell` (+ _array_element Cell))))

(fn `ShowCell`
  (params (Cell :type "IntPoint Structure"))
  (bind _position (`self.GridToWorld` Cell))
  (`SceneComponent.K2_SetWorldLocation` (`self.Highlight`) (+ _position (0.0 0.0 2.0)) false false)
  (bind _ok (`self.CanBuild` Cell))
  (if _ok
    (`PrimitiveComponent.SetMaterial` (`self.Highlight`) 0 (`self.GreenMaterial`))
    (else
      (`PrimitiveComponent.SetMaterial` (`self.Highlight`) 0 (`self.RedMaterial`)))))

(fn `ShowPreview`
  (params (Cell :type "IntPoint Structure") (Yaw :type "Float (double-precision)") (Mesh :type "StaticMesh Object Reference"))
  (`StaticMeshComponent.SetStaticMesh` (`self.Preview`) Mesh)
  (bind _position (`self.GridToWorld` Cell))
  (`SceneComponent.K2_SetWorldLocation` (`self.Preview`) (+ _position (0.0 0.0 50.0)) false false)
  (`SceneComponent.K2_SetWorldRotation` (`self.Preview`) (`KismetMathLibrary.MakeRotator` 0.0 0.0 Yaw) false false))

(fn `UserConstructionScript`)

(fn `WorldToGrid`
  (params (Position :type "Vector Structure"))
  (returns (Cell :type "IntPoint Structure"))
  (bind (_returnvalue_x _returnvalue_y) (`KismetMathLibrary.BreakVector` (`self.K2_GetActorLocation`)))
  (return (make `IntPoint` (`KismetMathLibrary.FFloor` (/ (- Position_X _returnvalue_x) (`self.CellSize`))) (`KismetMathLibrary.FFloor` (/ (- Position_Y _returnvalue_y) (`self.CellSize`))))))
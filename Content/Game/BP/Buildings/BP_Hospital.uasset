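; BP_Hospital is a building Blueprint that supplies happiness based on how many houses stand near it.
; GetHapiness scans all BP_House actors, counts those within Radius of the hospital, and returns that count times HappinessPerHouse.
; The count is rebuilt from the full actor list on every call.
; The event graph has no active logic, and the construction script only calls its parent.
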(fn `GetHapiness`
  (returns (Hapiness :type Integer))
  (set `self.NearbyHouses` 0)
  (bind _outactors (`GameplayStatics.GetAllActorsOfClass` "/Game/Game/BP/Buildings/BP_House.BP_House_C"))
  (for _array_element _outactors
    (if (<= (`self.GetDistanceTo` _array_element) (`self.Radius`))
      (set `self.NearbyHouses` (+ (`self.NearbyHouses`) 1))))
  (return (* (`self.NearbyHouses`) (`self.HappinessPerHouse`))))

(fn `UserConstructionScript`
  (`parent.UserConstructionScript`))
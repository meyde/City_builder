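; BP_Building is a data-driven building whose type is chosen by a row name.
; On BeginPlay it looks up that row in DT_Buildings, caches it as Info and applies the row's mesh to its Body component.
; GetIncome returns the income from Info, while GetResident and GetHapiness return only zero.
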(event `self.ReceiveBeginPlay`
  (bind _returnvalue (`|GetDataTableRow` "/Game/Game/Data/DT_Buildings.DT_Buildings" (`self.RowName`))
    (:`then`
      (bind _output_get (set `self.Info` _returnvalue))
      (`StaticMeshComponent.SetStaticMesh` (`self.Body`) (`.Mesh_5_6F616774494482E23066D7A65FA127F3` (break `/Game/Game/Data/S_Building` _output_get))))))

(fn `GetHapiness`
  (returns (Hapiness :type Integer))
  (return 0))

(fn `GetIncome`
  (returns (Income :type Integer))
  (return (`.Income_11_ECFAD36348C916757CF1DCB40A43C446` (break `/Game/Game/Data/S_Building` (`self.Info`)))))

(fn `GetResident`
  (returns (Residents :type Integer))
  (return 0))

(fn `UserConstructionScript`)
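; BP_Road is a grid-based road tile actor that reshapes itself to connect with neighbouring roads.
; UpdateShape takes a Grid and queries IsRoad on the four orthogonal neighbours of the actor's Cell.
; Each result toggles the visibility of a matching arm component (X+, X-, Y+, Y-), so straights, corners and junctions come from one Blueprint.
; The event graph and construction script add no logic of their own.
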(fn `UpdateShape`
  (params (Grid :type "/Game/Game/BP/Grid/BP_GridManager Object Reference"))
  (bind _road (`/Game/Game/BP/Grid/BP_GridManager.IsRoad` Grid (+ (make `IntPoint` 1) (`self.Cell`))))
  (`SceneComponent.SetVisibility` (`self.ArmXPlus`) _road false)
  (bind _road_2 (`/Game/Game/BP/Grid/BP_GridManager.IsRoad` Grid (+ (make `IntPoint` -1) (`self.Cell`))))
  (`SceneComponent.SetVisibility` (`self.ArmXMinus`) _road_2 false)
  (bind _road_3 (`/Game/Game/BP/Grid/BP_GridManager.IsRoad` Grid (+ (make `IntPoint` 0 1) (`self.Cell`))))
  (`SceneComponent.SetVisibility` (`self.ArmYPlus`) _road_3 false)
  (bind _road_4 (`/Game/Game/BP/Grid/BP_GridManager.IsRoad` Grid (+ (make `IntPoint` 0 -1) (`self.Cell`))))
  (`SceneComponent.SetVisibility` (`self.ArmYMinus`) _road_4 false))

(fn `UserConstructionScript`
  (`parent.UserConstructionScript`))